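; Monster spawner component that spawns BP_Monster AI running BT_Monster around its owning actor.
; On BeginPlay a looping timer calls DoSpawn each second and clears itself once the spawn count passes its limit, ten monsters from zero.
; GetRandomLocation picks a point on a horizontal circle of twice Radius around the owner.
; IsCanSpawn line-traces downward for world geometry, but nothing in these graphs calls it.
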(event `self.ReceiveBeginPlay`
  (`KismetSystemLibrary.K2_SetTimer` null "DoSpawn" 1.0 true))

(fn `DoSpawn`
  (set `self.Location` (`self.GetRandomLocation`))
  (set `self.SpawnCount` (+ (`self.SpawnCount`) 1.0))
  (`AIBlueprintHelperLibrary.SpawnAIFromClass` "/Game/SurvivalGame/Monster/BP_Monster.BP_Monster_C" "/Game/SurvivalGame/Monster/BT_Monster.BT_Monster" (`self.Location`) (struct) false null)
  (if (> (`self.SpawnCount`) 9.0)
    (`KismetSystemLibrary.K2_ClearTimer` null "DoSpawn")))

(fn `GetRandomLocation`
  (returns (RandCircle :type "Vector Structure"))
  (locals (Rand :type "Float (double-precision)"))
  (bind _returnvalue (* (`self.Radius`) 2.0))
  (bind _output_get (set `local.Rand` (`KismetMathLibrary.RandomFloatInRange` 0.0 360.0)))
  (return (+ (`Actor.K2_GetActorLocation` (`self.GetOwner`)) (`KismetMathLibrary.MakeVector` (* (`KismetMathLibrary.Cos` _output_get) _returnvalue) (* (`KismetMathLibrary.Sin` _output_get) _returnvalue)))))

(fn `IsCanSpawn`
  (params (Location :type "Vector Structure"))
  (returns (IsCan :type Boolean))
  (bind (_outhit _returnvalue) (`KismetSystemLibrary.LineTraceSingleForObjects` Location (- Location (0.0 0.0 100.0)) (`|MakeArray` "ObjectTypeQuery1" "ObjectTypeQuery2" :!type "EObjectTypeQuery Enum")))
  (return _returnvalue))