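; Player state Blueprint for a survival game that tracks the player's health.
; AddDamage subtracts damage while HP is above zero, broadcasts current and max HP through an UpdateHP dispatcher, and fires a Death dispatcher once HP reaches zero or below.
; SetHP resets current HP to a hardcoded value, independent of MaxHP and without broadcasting.
; The event graph and construction script contain no logic.
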(fn `AddDamage`
  (params (Damage :type "Float (double-precision)"))
  (if (> (`self.CurHP`) 0.0)
    (bind _output_get (set `self.CurHP` (- (`self.CurHP`) Damage)))
    (`self.EventDispatcherUpdateHP` _output_get (`self.MaxHP`))
    (if (<= (`self.CurHP`) 0.0)
      (`self.EventDispatcherDeath`))))

(fn `SetHP`
  (set `self.CurHP` 100.0))

(fn `UserConstructionScript`)